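; Sliding door Blueprint for the procedural dungeon that moves its Door component vertically to open and close.
; OpenDoor runs only when unlocked and closed, lowering the door by timeline, while CloseDoor requires it open and raises it with a second timeline.
; Both lerp from a stored Z, cached at BeginPlay, toward fixed relative heights, updating that Z and the open state on finish.
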(event Custom|OpenDoor
  (bind _door (Variables|Default|GetDoor))
  (bind _relativelocation (Variables|/Script/Engine.SceneComponent|GetRelativeLocation _door))
  ;[0.1946 1 0.01938] Open Door with animation
  (if (Variables|Default|GetisUnlocked)
    (if (not (Variables|Default|GetisOpen))
      (bind _dooropen (Timeline|OpenDoorTimeline PlayFromStart)
        (:Update
          (Transformation|SetRelativeLocation _door (Math|Vector|MakeVector (.x _relativelocation) (.y _relativelocation) (Math|Float|Lerp (Variables|Default|GetLast%20Relative%20Location%20Z) -6e+02 _dooropen)) false false))
        (:Finished
          (Variables|Default|SetLast%20Relative%20Location%20Z (.z _relativelocation))
          (Variables|Default|SetisOpen true))))))

(event Custom|CloseDoor
  (bind _door (Variables|Default|GetDoor))
  (bind _relativelocation (Variables|/Script/Engine.SceneComponent|GetRelativeLocation _door))
  ;[0.1946 1 0.01938] Close door with animation
  (if (Variables|Default|GetisOpen)
    (bind _dooropen (Timeline|Timeline PlayFromStart)
      (:Update
        (Transformation|SetRelativeLocation _door (Math|Vector|MakeVector (.x _relativelocation) (.y _relativelocation) (Math|Float|Lerp (Variables|Default|GetLast%20Relative%20Location%20Z) 6e+02 _dooropen)) false false))
      (:Finished
        (Variables|Default|SetLast%20Relative%20Location%20Z (.z _relativelocation))
        (Variables|Default|SetisOpen false)))))

(event EventBeginPlay
  (Variables|Default|SetLast%20Relative%20Location%20Z (.z (Variables|/Script/Engine.SceneComponent|GetRelativeLocation (Variables|Default|GetDoor)))))

(fn ConstructionScript)